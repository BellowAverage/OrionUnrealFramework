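; BP_XChara is an Orion character Blueprint that carries a primary weapon between back and hand and fires it.
; BeginPlay spawns the weapon onto the back socket; SpawnWeaponActor and RemoveWeaponActor only reattach that instance to hand or back.
; GetAttachBackTransformation stores offsets, handedness and long-range attack timings, while firing passes target and forward-offset muzzle location to the weapon.
; Shoulder cargo-copying logic remains but is disconnected.
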(event Custom|InitWeaponActor
  (bind _returnvalue (Game|SpawnActorfromClass (Variables|Default|GetPrimaryWeaponClass) (Math|Transform|MakeTransform "0, 0, 0" "0, 0, 0" "1.000000,1.000000,1.000000") "Undefined" "MultiplyWithRoot" self 0))
  (bind _output_get (Variables|Default|SetPrimaryWeaponInstance _returnvalue))
  (Transformation|AttachComponentToComponent _output_get (Variables|Default|GetSocket_WeaponBack) "None" "KeepRelative" "KeepRelative" "KeepRelative" true)
  (Transformation|SetRelativeTransform (Variables|/Script/Engine.Actor|GetRootComponent (Variables|Default|GetPrimaryWeaponInstance)) (Variables|Default|GetBackAttachTransformationOffset) false false)
  (Variables|Default|SetAttackFrequencyLongRange (Variables|Default|GetWeaponAttackFrequencyLongRange))
  (Variables|Default|SetAttackTriggerTimeLongRange (Variables|Default|GetWeaponTriggerTimeLongRange)))

(event Custom|GetAttachBackTransformation
  (params (BackAttachTransformationOffset :type Transform) (HandAttachTransformationOffset :type Transform) (GetbIsRightHandWeapon :type Boolean) (SpawnFrontOffset :type Float%20%28double-precision%29) (AttackFrequencyLongRange :type Float%20%28double-precision%29) (AttackTriggerTimeLongRange :type Float%20%28double-precision%29))
  (Variables|Default|SetBackAttachTransformationOffset BackAttachTransformationOffset)
  (Variables|Default|SetHandAttachTransformationOffset HandAttachTransformationOffset)
  (Variables|Default|SetbIsRightHandWeapon GetbIsRightHandWeapon)
  (Variables|Default|SetSpawnFrontOffset SpawnFrontOffset)
  (Variables|Default|SetWeaponAttackFrequencyLongRange AttackFrequencyLongRange)
  (Variables|Default|SetWeaponTriggerTimeLongRange AttackTriggerTimeLongRange))

(event EventBeginPlay
  (|CallParentFunction)
  (CallFunction|InitWeaponActor)
  (Transformation|AttachComponentToComponent (Variables|Default|GetSocket_ShoulderR) (Variables|Default|GetTorso) "clavicle_r" "KeepRelative" "KeepRelative" "KeepRelative" true))

(event Collision|EventActorBeginOverlap
  (params (OtherActor :type Actor%20Object%20Reference)))

(event EventRemoveWeaponActor
  (Transformation|AttachComponentToComponent (Variables|Default|GetPrimaryWeaponInstance) (Variables|Default|GetSocket_WeaponBack) "None" "KeepRelative" "KeepRelative" "KeepRelative" true)
  (Transformation|SetRelativeTransform (Variables|/Script/Engine.Actor|GetRootComponent (Variables|Default|GetPrimaryWeaponInstance)) (Variables|Default|GetBackAttachTransformationOffset) false false))

(event EventSpawnWeaponActor
  (Transformation|SetRelativeTransform (Variables|/Script/Engine.Actor|GetRootComponent (Variables|Default|GetPrimaryWeaponInstance)) (Math|Transform|MakeTransform "0, 0, 0" "0, 0, 0" "1.000000,1.000000,1.000000") false false)
  (if (Variables|Default|GetbIsRightHandWeapon)
    (Transformation|AttachComponentToComponent (Variables|Default|GetPrimaryWeaponInstance) (Variables|Default|GetWeapon_R) "None" "KeepRelative" "KeepRelative" "KeepRelative" true)
    (else
      (Transformation|AttachComponentToComponent (Variables|Default|GetPrimaryWeaponInstance) (Variables|Default|GetWeapon_L) "None" "KeepRelative" "KeepRelative" "KeepRelative" true))))

(event EventTick
  (params (DeltaSeconds :type Float%20%28single-precision%29)))

(event EventSpawnOrionBulletActor
  (params (TargetLocation :type Vector%20%28by%20ref%29 :default "0, 0, 0") (MuzzleLocation :type Vector%20%28by%20ref%29 :default "0, 0, 0"))
  (Class|OrionWeapon|SpawnOrionBulletActor (Variables|Default|GetPrimaryWeaponInstance) TargetLocation (+ "0.000000,0.000000,5.000000" (* (Transformation|GetActorForwardVector) (Variables|Default|GetSpawnFrontOffset)) (Transformation|GetActorLocation (Variables|Default|GetPrimaryWeaponInstance)))))

(fn ConstructionScript
  (|CallParentFunction))